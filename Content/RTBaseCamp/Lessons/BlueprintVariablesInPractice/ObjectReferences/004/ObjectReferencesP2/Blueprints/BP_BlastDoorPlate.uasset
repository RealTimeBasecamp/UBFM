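; BP_BlastDoorPlate is a pressure plate that opens a referenced blast door while something overlaps its box and closes it when the overlap ends.
; Begin and end overlap call DoorOpening on the door reference with true or false.
; They also play or reverse a timeline that lerps the pad from its starting relative location, saved at BeginPlay, to a fixed offset.
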(event OnComponentBeginOverlap(OverlapBox)
  (params (OverlappedComponent :type Primitive%20Component%20Object%20Reference) (OtherActor :type Actor%20Object%20Reference) (OtherComp :type Primitive%20Component%20Object%20Reference) (OtherBodyIndex :type Integer) (bFromSweep :type Boolean) (SweepResult :type Hit%20Result%20Structure%20%28by%20ref%29))
  (Default|DoorOpening (Variables|Default|GetDoorReference) true)
  (bind _padslidefloatlerp (Timeline|PressurePlateTimeline Play)
    (:Update
      (Transformation|SetRelativeLocation (Variables|Default|GetPad) (Math|Vector|Lerp(Vector) (Variables|Default|GetRelative%20Location) "0.000000,0.000000,4.000000" _padslidefloatlerp) false false))))

(event OnComponentEndOverlap(OverlapBox)
  (params (OverlappedComponent :type Primitive%20Component%20Object%20Reference) (OtherActor :type Actor%20Object%20Reference) (OtherComp :type Primitive%20Component%20Object%20Reference) (OtherBodyIndex :type Integer))
  (Default|DoorOpening (Variables|Default|GetDoorReference) false)
  (bind _padslidefloatlerp (Timeline|PressurePlateTimeline Reverse)
    (:Update
      (Transformation|SetRelativeLocation (Variables|Default|GetPad) (Math|Vector|Lerp(Vector) (Variables|Default|GetRelative%20Location) "0.000000,0.000000,4.000000" _padslidefloatlerp) false false))))

(event EventBeginPlay
  (Variables|Default|SetRelative%20Location (Variables|/Script/Engine.SceneComponent|GetRelativeLocation (Variables|Default|GetPad))))

(fn ConstructionScript)