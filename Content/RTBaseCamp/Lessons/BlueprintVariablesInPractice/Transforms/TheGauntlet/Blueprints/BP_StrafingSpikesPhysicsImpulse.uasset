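; Strafing spike hazard that moves between two points and knocks characters away on contact.
; On BeginPlay it caches the start and end debug sphere locations, waits StrafeDelay, then a Timeline lerps the spike mesh between them without sweep.
; Box overlap finds the other actor's CharacterMovementComponent and applies a large mass-dependent horizontal impulse directed away from the box.
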(event OnComponentBeginOverlap(Box)
  (params (OverlappedComponent :type Primitive%20Component%20Object%20Reference) (OtherActor :type Actor%20Object%20Reference) (OtherComp :type Primitive%20Component%20Object%20Reference) (OtherBodyIndex :type Integer) (bFromSweep :type Boolean) (SweepResult :type Hit%20Result%20Structure%20%28by%20ref%29))
  (bind _returnvalue (Actor|GetComponentbyClass OtherActor "/Script/Engine.CharacterMovementComponent"))
  ;[0.9647 0.5711 0.01681 0.5] Added Physics Impulse
  (Utilities|IsValid _returnvalue
    (:Is%20Valid
      (Physics|AddImpulse _returnvalue (* (Math|Vector|GetUnitDirection(Vector) (Transformation|GetWorldLocation (Variables|/Script/Engine.MovementComponent|GetUpdatedPrimitive _returnvalue)) (Transformation|GetWorldLocation OverlappedComponent)) "-1500000.000000,-1500000.000000,0.000000") false))))

(event EventBeginPlay
  (Variables|Default|SetStrafeStartLoc (Transformation|GetWorldLocation (Variables|Default|GetStartLocDebugSphere)))
  (Variables|Default|SetStrafeEndLoc (Transformation|GetWorldLocation (Variables|Default|GetEndLocDebugSphere)))
  (Utilities|FlowControl|Delay (Variables|Default|GetStrafeDelay))
  (bind _strafelerpamount (Timeline|Timeline PlayFromStart)
    (:Update
      (Transformation|SetWorldLocation (Variables|Default|GetSM_StrafingSpikes) (Math|Vector|Lerp(Vector) (Math|Vector|MakeVector (.x (Variables|Default|GetStrafeStartLoc)) (.y (Variables|Default|GetStrafeStartLoc)) (.z (Variables|Default|GetStrafeStartLoc))) (Math|Vector|MakeVector (.x (Variables|Default|GetStrafeEndLoc)) (.y (Variables|Default|GetStrafeEndLoc)) (.z (Variables|Default|GetStrafeEndLoc))) _strafelerpamount) false false))))

(fn ConstructionScript)