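; BP_EnumCube is a Crash Bandicoot-style crate whose MeshType enum selects its mesh and behaviour: Coin, TNT or Nitro.
; Coin crates bounce the player from the top box, breaking when damaged or out of bounces.
; Damage or side-box overlap starts TNT's pulsing timeline countdown or detonates Nitro immediately.
; Explosions fire a radial impulse and apply radial damage, which can chain to other crates, before self-destruction.
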(event OnComponentBeginOverlap(OutsideCollisionBox)
  (params (OverlappedComponent :type Primitive%20Component%20Object%20Reference) (OtherActor :type Actor%20Object%20Reference) (OtherComp :type Primitive%20Component%20Object%20Reference) (OtherBodyIndex :type Integer) (bFromSweep :type Boolean) (SweepResult :type Hit%20Result%20Structure%20%28by%20ref%29))
  (bind _startingworldscale (Variables|Default|GetStartingWorldScale))
  (bind _staticmesh (Variables|Default|GetStaticMesh))
  (if (not (== (Utilities|GetClass OtherActor) "BP_EnumCube_C"))
    (switch Utilities|FlowControl|Switch|SwitchonECubeType (Variables|Default|GetMeshType)
      (:NewEnumerator1
        (if (not (Variables|Default|GetExplosionInitiated))
          (Variables|Default|SetExplosionInitiated true)
          (Audio|Components|Audio|Play (Variables|Default|GetTNTCountdownSFX) 0.0)
          (bind _newtrack_2 (Timeline|TnTTimeline PlayFromStart)
            (:Update
              (Transformation|SetWorldScale3D (Variables|Default|GetStaticMesh) (Math|Vector|Lerp(Vector) _startingworldscale (* _startingworldscale "1.100000,1.100000,1.100000") _newtrack_2)))
            (:Finished
              (Components|Activation|Activate (Variables|Default|GetP_Explosion) true :!label _label)
              (Class|RadialForceComponent|FireImpulse (Variables|Default|GetRadialForce))
              (Audio|Components|Audio|Play (Variables|Default|GetCreateExplosion) 0.0)
              (Variables|Default|SetHasExploded true)
              (Development|SetHiddeninGame _staticmesh true false)
              (Game|Damage|ApplyRadialDamage 1.0 (Transformation|GetWorldLocation _staticmesh) 2.5e+02 0 0 0 0 false "ECC_Visibility")
              (Utilities|FlowControl|Delay 1.0)
              (Actor|DestroyActor)))))
      (:NewEnumerator2
        (goto _label)))))

(event OnComponentBeginOverlap(TopCollisionBox)
  (params (OverlappedComponent :type Primitive%20Component%20Object%20Reference) (OtherActor :type Actor%20Object%20Reference) (OtherComp :type Primitive%20Component%20Object%20Reference) (OtherBodyIndex :type Integer) (bFromSweep :type Boolean) (SweepResult :type Hit%20Result%20Structure%20%28by%20ref%29))
  (switch Utilities|FlowControl|Switch|SwitchonECubeType (Variables|Default|GetMeshType)
    (:NewEnumerator0
      (if (== (Variables|Default|GetBounceCount) 0)
        (CallFunction|CoinCrateExplode)
        (else
          ;[1 1 1] CoinCrate
          (if (== (Utilities|GetClass OtherActor) "/Game/FirstPerson/Blueprints/BP_FirstPersonCharacter.BP_FirstPersonCharacter_C")
            (Physics|AddImpulse (Actor|GetComponentbyClass (Game|Player|GetPlayerPawn 0) "/Script/Engine.CharacterMovementComponent") "0.000000,0.000000,75000.000000" false)
            (Math|Integer|DecrementInt (Variables|Default|GetBounceCount)
              (:%20%20
                (Audio|Components|Audio|Play (Variables|Default|GetBounceSFX) 0.0)))))))))

(event Custom|CoinCrateExplode
  (if (not (Variables|Default|GetHasExploded))
    (Audio|Components|Audio|Play (Variables|Default|GetCrateBreakSFX) 0.0)
    (Variables|Default|SetHasExploded true)
    (Collision|SetCollisionEnabled (Variables|Default|GetStaticMesh) "NoCollision")
    (Physics|AddImpulse (Actor|GetComponentbyClass (Game|Player|GetPlayerPawn 0) "/Script/Engine.CharacterMovementComponent") "0.000000,0.000000,75000.000000" false)
    (Components|Activation|Activate (Variables|Default|GetFXS_WumpaFruit) false)
    (Development|SetHiddeninGame (Variables|Default|GetStaticMesh) true false)
    (Utilities|FlowControl|Delay 6.0)
    (Actor|DestroyActor)))

(event EventBeginPlay
  (Variables|Default|SetStartingWorldScale (Transformation|GetWorldScale (Variables|Default|GetStaticMesh))))

(event Game|Damage|EventAnyDamage
  (params (Damage :type Float%20%28single-precision%29) (DamageType :type Damage%20Type%20Object%20Reference) (InstigatedBy :type Controller%20Object%20Reference) (DamageCauser :type Actor%20Object%20Reference))
  (bind _startingworldscale (Variables|Default|GetStartingWorldScale))
  (bind _staticmesh (Variables|Default|GetStaticMesh))
  (if (not (Variables|Default|GetHasExploded))
    (Development|PrintString (Utilities|GetDisplayName DamageCauser))
    (if (Utilities|Enum|Equal(Enum) (Variables|Default|GetMeshType) "NewEnumerator0")
      (CallFunction|CoinCrateExplode)
      (else
        (switch Utilities|FlowControl|Switch|SwitchonECubeType (Variables|Default|GetMeshType)
          (:NewEnumerator1
            (if (not (Variables|Default|GetExplosionInitiated))
              (Variables|Default|SetExplosionInitiated true)
              (Audio|Components|Audio|Play (Variables|Default|GetTNTCountdownSFX) 0.0)
              (bind _newtrack_2 (Timeline|TnTTimeline PlayFromStart)
                (:Update
                  (Transformation|SetWorldScale3D (Variables|Default|GetStaticMesh) (Math|Vector|Lerp(Vector) _startingworldscale (* _startingworldscale "1.100000,1.100000,1.100000") _newtrack_2)))
                (:Finished
                  (Components|Activation|Activate (Variables|Default|GetP_Explosion) true :!label _label)
                  (Class|RadialForceComponent|FireImpulse (Variables|Default|GetRadialForce))
                  (Audio|Components|Audio|Play (Variables|Default|GetCreateExplosion) 0.0)
                  (Variables|Default|SetHasExploded true)
                  (Development|SetHiddeninGame _staticmesh true false)
                  (Game|Damage|ApplyRadialDamage 1.0 (Transformation|GetWorldLocation _staticmesh) 2.5e+02 0 0 0 0 false "ECC_Visibility")
                  (Utilities|FlowControl|Delay 1.0)
                  (Actor|DestroyActor)))))
          (:NewEnumerator2
            (goto _label)))))))

(fn ConstructionScript
  (bind _staticmesh (Variables|Default|GetStaticMesh))
  (switch Utilities|FlowControl|Switch|SwitchonECubeType (Variables|Default|GetMeshType)
    (:NewEnumerator0
      (Components|StaticMesh|SetStaticMesh _staticmesh "/Game/RTBaseCamp/Lessons/BlueprintVariablesInPractice/ENUMS/FurtherUsesOfENUMS/Meshes/SM_JumpCrate.SM_JumpCrate"))
    (:NewEnumerator1
      (Components|StaticMesh|SetStaticMesh _staticmesh "/Game/RTBaseCamp/Lessons/BlueprintVariablesInPractice/ENUMS/FurtherUsesOfENUMS/Meshes/SM_TNTCrate2.SM_TNTCrate2"))
    (:NewEnumerator2
      (Components|StaticMesh|SetStaticMesh _staticmesh "/Game/RTBaseCamp/Lessons/BlueprintVariablesInPractice/ENUMS/FurtherUsesOfENUMS/Meshes/SM_NitroCrate2.SM_NitroCrate2")))
  (Components|Timeline|SetPlayRate (Variables|Default|GetTnTTimeline) 3.0))