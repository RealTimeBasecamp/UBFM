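; BP_Cube is an enum lesson actor: a configurable shape that fires a radial impulse when something overlaps its box.
; The construction script uses the MeshType enum to pick a cube, sphere or cone mesh, and MeshColour to set both material and scale.
; Box overlap triggers the RadialForce component.
; Unconnected leftover logic would hide the actor or launch the player upward for cubes, but never runs.
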(event OnComponentBeginOverlap(Box)
  (params (OverlappedComponent :type Primitive%20Component%20Object%20Reference) (OtherActor :type Actor%20Object%20Reference) (OtherComp :type Primitive%20Component%20Object%20Reference) (OtherBodyIndex :type Integer) (bFromSweep :type Boolean) (SweepResult :type Hit%20Result%20Structure%20%28by%20ref%29))
  (Class|RadialForceComponent|FireImpulse (Variables|Default|GetRadialForce)))

(fn ConstructionScript
  (bind _staticmesh (Variables|Default|GetStaticMesh))
  (switch Utilities|FlowControl|Switch|SwitchonEMeshType (Variables|Default|GetMeshType)
    (:NewEnumerator0
      (Components|StaticMesh|SetStaticMesh _staticmesh "/Game/StarterContent/Shapes/Shape_Cube.Shape_Cube"))
    (:NewEnumerator1
      (Components|StaticMesh|SetStaticMesh _staticmesh "/Game/StarterContent/Shapes/Shape_Sphere.Shape_Sphere"))
    (:NewEnumerator2
      (Components|StaticMesh|SetStaticMesh _staticmesh "/Game/StarterContent/Shapes/Shape_Cone.Shape_Cone")))
  (Rendering|Material|SetMaterial (Variables|Default|GetStaticMesh) 0 (Utilities|Select :Index (Variables|Default|GetMeshColour) :NewEnumerator0 (Variables|Default|GetRedMat) :NewEnumerator1 (Variables|Default|GetGreenMat) :NewEnumerator2 (Variables|Default|GetBlueMat)))
  (Transformation|SetRelativeScale3D (Variables|Default|GetStaticMesh) (Utilities|Select :Index (Variables|Default|GetMeshColour) :NewEnumerator0 (Math|Vector|MakeVector 1.0 1.0 1.0) :NewEnumerator1 (Math|Vector|MakeVector 2.0 2.0 2.0) :NewEnumerator2 (Math|Vector|MakeVector 5.0 5.0 5.0))))