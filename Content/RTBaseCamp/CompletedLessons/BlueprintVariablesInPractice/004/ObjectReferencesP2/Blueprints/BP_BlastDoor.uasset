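; BP_BlastDoor is a lesson blast door that slides open or closed, with animated lock parts, through a DoorOpening event taking a boolean.
; BeginPlay caches the world locations of the door, bolt, and top and bottom lock slides.
; One timeline plays or reverses, using separate lock and door tracks to lerp the parts from those locations.
; Offsets are hardcoded along world axes, so movement ignores the actor's rotation.
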(event Custom|DoorOpening
  (params (IsDoorOpening :type Boolean))
  (bind _lockslidebottomstartloc (Variables|Default|GetLockSlideBottomStartLoc))
  (bind _doorstartinglocation (Variables|Default|GetDoorStartingLocation))
  (bind _boltstartinglocation (Variables|Default|GetBoltStartingLocation))
  (bind _lockslidetopstartloc (Variables|Default|GetLockSlideTopStartLoc))
  (if IsDoorOpening
    (bind (_direction _dooropeninglerp _lockopeningtimeline) (Timeline|BooleanDoorSlideUp Play)
      (:Update
        (Transformation|SetWorldLocation (Variables|Default|GetSM_BlastDoorLock_SM_BlastDoorBolt) (Math|Vector|MakeVector (Math|Float|Lerp (.x _boltstartinglocation) (- (.x _boltstartinglocation) 65.0) _lockopeningtimeline) (.y _boltstartinglocation) (.z _boltstartinglocation)) false false)
        (Transformation|SetWorldLocation (Variables|Default|GetSM_BlastDoorLockSlideTop) (Math|Vector|MakeVector (.x _lockslidetopstartloc) (.y _lockslidetopstartloc) (Math|Float|Lerp (.z _lockslidetopstartloc) (+ (.z _lockslidetopstartloc) 65.0) _lockopeningtimeline)) false false)
        (Transformation|SetWorldLocation (Variables|Default|GetSM_BlastDoorLockSlideBottom) (Math|Vector|MakeVector (.x _lockslidebottomstartloc) (.y _lockslidebottomstartloc) (Math|Float|Lerp (.z _lockslidebottomstartloc) (- (.z _lockslidebottomstartloc) 65.0) _lockopeningtimeline)) false false)
        (Transformation|SetWorldLocation (Variables|Default|GetSM_BooleanDoor) (Math|Vector|MakeVector (.x _doorstartinglocation) (Math|Float|Lerp (.y _doorstartinglocation) (+ (.y _doorstartinglocation) 1e+03) _dooropeninglerp) (.z _doorstartinglocation)) false false)))
    (else
      (Timeline|BooleanDoorSlideUp Reverse))))

(event EventBeginPlay
  (Variables|Default|SetDoorStartingLocation (Transformation|GetWorldLocation (Variables|Default|GetSM_BooleanDoor)))
  (Variables|Default|SetBoltStartingLocation (Transformation|GetWorldLocation (Variables|Default|GetSM_BlastDoorLock_SM_BlastDoorBolt)))
  (Variables|Default|SetLockSlideTopStartLoc (Transformation|GetWorldLocation (Variables|Default|GetSM_BlastDoorLockSlideTop)))
  (Variables|Default|SetLockSlideBottomStartLoc (Transformation|GetWorldLocation (Variables|Default|GetSM_BlastDoorLockSlideBottom))))

(fn ConstructionScript)