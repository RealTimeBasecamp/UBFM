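; BP_PresurePlateDoor is a lesson door that slides open and closed, with its name indicating pressure plate control.
; It caches the door mesh's world location on BeginPlay.
; The DoorOpening event takes a boolean that plays or reverses the BooleanDoorSlideUp timeline, which lerps the mesh along world Y from that cached position.
; Despite the timeline's name, the Z position stays fixed.
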(event Custom|DoorOpening
  (params (IsDoorOpening :type Boolean))
  (bind _doorstartinglocation (Variables|Default|GetDoorStartingLocation))
  (if IsDoorOpening
    (bind _dooropeninglerp (Timeline|BooleanDoorSlideUp Play)
      (:Update
        (Transformation|SetWorldLocation (Variables|Default|GetSM_BooleanDoor) (Math|Vector|MakeVector (.x _doorstartinglocation) (Math|Float|Lerp (.y _doorstartinglocation) (+ (.y _doorstartinglocation) 1301.0) _dooropeninglerp) (.z _doorstartinglocation)) false false)))
    (else
      (Timeline|BooleanDoorSlideUp Reverse))))

(event EventBeginPlay
  (Variables|Default|SetDoorStartingLocation (Transformation|GetWorldLocation (Variables|Default|GetSM_BooleanDoor))))

(fn ConstructionScript)