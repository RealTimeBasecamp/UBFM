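; Swinging spike hazard that sweeps around a pivot and knocks characters away on contact.
; The construction script sets the pivot's starting roll; after a configurable delay, a rate-scaled timeline lerps it to the mirrored angle using its scale track.
; When the blade body overlaps an actor with a CharacterMovementComponent, it prints a debug string and applies a large horizontal, mass-dependent impulse pointing away from the blade.
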(event OnComponentBeginOverlap(BladeBody)
  (params (OverlappedComponent :type Primitive%20Component%20Object%20Reference) (OtherActor :type Actor%20Object%20Reference) (OtherComp :type Primitive%20Component%20Object%20Reference) (OtherBodyIndex :type Integer) (bFromSweep :type Boolean) (SweepResult :type Hit%20Result%20Structure%20%28by%20ref%29))
  (bind _returnvalue (Actor|GetComponentbyClass OtherActor "/Script/Engine.CharacterMovementComponent"))
  ;[1 1 1] Uses Collision preset OverlapOnlyPawn
  (Utilities|IsValid _returnvalue
    (:Is%20Valid
      (Development|PrintString "Hello")
      (Physics|AddImpulse _returnvalue (* (Math|Vector|GetUnitDirection(Vector) (Transformation|GetWorldLocation (Variables|/Script/Engine.MovementComponent|GetUpdatedPrimitive _returnvalue)) (Transformation|GetWorldLocation OverlappedComponent)) "-1500000.000000,-1500000.000000,0.000000") false))))

(event EventBeginPlay
  (Components|Timeline|SetPlayRate (Variables|Default|GetRotateBladeTimeline) (Variables|Default|GetRotationSpeed))
  (Variables|Default|SetStartingRelativeRotation (Variables|/Script/Engine.SceneComponent|GetRelativeRotation (Variables|Default|GetRotationPivot)))
  (Utilities|FlowControl|Delay (Variables|Default|GetRotateDelay))
  (bind _slidingspikescale (Timeline|RotateBladeTimeline PlayFromStart)
    (:Update
      (Transformation|SetRelativeRotation (Variables|Default|GetRotationPivot) (Math|Rotator|MakeRotator (Math|Float|Lerp (.roll (Variables|Default|GetStartingRelativeRotation)) (+ (.roll (Variables|Default|GetStartingRelativeRotation)) (* (Variables|Default|GetRotationAmount) -2.0)) _slidingspikescale) (.pitch (Variables|Default|GetStartingRelativeRotation)) (.yaw (Variables|Default|GetStartingRelativeRotation))) false false))))

(fn ConstructionScript
  (bind _rotationpivot (Variables|Default|GetRotationPivot))
  (bind _relativerotation (Variables|/Script/Engine.SceneComponent|GetRelativeRotation _rotationpivot))
  (Transformation|SetRelativeRotation _rotationpivot (Math|Rotator|MakeRotator (Variables|Default|GetRotationAmount) (.pitch _relativerotation) (.yaw _relativerotation)) false false))