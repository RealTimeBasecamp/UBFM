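; BP_StrafingSpikes is a moving spike hazard from a transforms lesson that slides between two points set by debug spheres.
; On BeginPlay it stores both spheres' world locations, waits for a configurable delay, then plays a timeline.
; The timeline's alpha lerps the spike mesh's X and Y between those points while keeping its current Z, without sweep.
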(event EventBeginPlay
  (bind _sm_strafingspikes (Variables|Default|GetSM_StrafingSpikes))
  (bind _returnvalue (Transformation|GetWorldLocation _sm_strafingspikes))
  (Variables|Default|SetStrafeStartLoc (Transformation|GetWorldLocation (Variables|Default|GetStartLocDebugSphere)))
  (Variables|Default|SetStrafeEndLoc (Transformation|GetWorldLocation (Variables|Default|GetEndLocDebugSphere)))
  (Utilities|FlowControl|Delay (Variables|Default|GetStrafeDelay))
  (bind _strafelerpamount (Timeline|Timeline PlayFromStart)
    (:Update
      (Transformation|SetWorldLocation _sm_strafingspikes (Math|Vector|Lerp(Vector) (Math|Vector|MakeVector (.x (Variables|Default|GetStrafeStartLoc)) (.y (Variables|Default|GetStrafeStartLoc)) (.z _returnvalue)) (Math|Vector|MakeVector (.x (Variables|Default|GetStrafeEndLoc)) (.y (Variables|Default|GetStrafeEndLoc)) (.z _returnvalue)) _strafelerpamount) false false))))

(fn ConstructionScript)