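; Sliding spike trap, from a tutorial on transforms, that extends by scaling its mesh and knocks characters back.
; Timelines lerp relative scale from the value cached at BeginPlay, either looping or triggered by first-person character overlap with a cooldown and Y-length multiplier.
; An impulse box pushes movement components horizontally away, re-armed when the overlap timeline finishes.
; An unwired node shows the pitfall of lerping from current scale.
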(event OnComponentBeginOverlap(ImpulseBox)
  (params (OverlappedComponent :type Primitive%20Component%20Object%20Reference) (OtherActor :type Actor%20Object%20Reference) (OtherComp :type Primitive%20Component%20Object%20Reference) (OtherBodyIndex :type Integer) (bFromSweep :type Boolean) (SweepResult :type Hit%20Result%20Structure%20%28by%20ref%29))
  (bind _returnvalue (Actor|GetComponentbyClass OtherActor "/Script/Engine.CharacterMovementComponent"))
  ;[1 1 1] Explained later on in another tutorial
  (if (not (Variables|Default|GetImpulseReset))
    (Utilities|IsValid _returnvalue
      (:Is%20Valid
        (Variables|Default|SetImpulseReset true)
        (Physics|AddImpulse _returnvalue (* (Math|Vector|GetUnitDirection(Vector) (Transformation|GetWorldLocation (Variables|/Script/Engine.MovementComponent|GetUpdatedPrimitive _returnvalue)) (Transformation|GetWorldLocation OverlappedComponent)) "-1500000.000000,-1500000.000000,0.000000") false)))))

(event OnComponentBeginOverlap(ActivateSpikesBox)
  (params (OverlappedComponent :type Primitive%20Component%20Object%20Reference) (OtherActor :type Actor%20Object%20Reference) (OtherComp :type Primitive%20Component%20Object%20Reference) (OtherBodyIndex :type Integer) (bFromSweep :type Boolean) (SweepResult :type Hit%20Result%20Structure%20%28by%20ref%29))
  (if (== (Utilities|GetClass OtherActor) "/Game/FirstPerson/Blueprints/BP_FirstPersonCharacter.BP_FirstPersonCharacter_C")
    (if (not (Variables|Default|GetIsCoolingDown))
      (Variables|Default|SetIsCoolingDown true)
      (bind _spikescale (Timeline|SpikeScaleTimelineOverlap PlayFromStart)
        (:Update
          (Transformation|SetRelativeScale3D (Variables|Default|GetSM_SlidingSpikes) (Math|Vector|Lerp(Vector) (Variables|Default|GetSpikesStartingScale) (Math|Vector|MakeVector 1.0 (Variables|Default|GetSpikeLengthMultiplier) 1.0) _spikescale)))
        (:Finished
          (Variables|Default|SetIsCoolingDown false)
          (Variables|Default|SetImpulseReset false))))))

(event EventBeginPlay
  ;[0.000304 0.3813 0.8632 0.5] Set Starting Scale from Relative
  (Variables|Default|SetSpikesStartingScale (Variables|/Script/Engine.SceneComponent|GetRelativeScale3D (Variables|Default|GetSM_SlidingSpikes)))
  ;[0.2961 0 0 0.5] Check if the spikes are looping
  (if (Variables|Default|GetIsLooping)
    ;[0.9647 0.5711 0.01681 0.5] Set Relative Scale
    (bind _spikescale (Timeline|SpikeScaleTimelineLooping PlayFromStart)
      (:Update
        (Transformation|SetRelativeScale3D (Variables|Default|GetSM_SlidingSpikes) (Math|Vector|Lerp(Vector) (Variables|Default|GetSpikesStartingScale) "1.000000,1.000000,1.000000" _spikescale))))))

(fn ConstructionScript)