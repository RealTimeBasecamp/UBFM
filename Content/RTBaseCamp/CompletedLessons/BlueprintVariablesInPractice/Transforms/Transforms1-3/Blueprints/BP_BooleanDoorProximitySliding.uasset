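; A lesson Blueprint for a proximity door that slides upward once when the first-person character enters its collision box.
; BeginPlay caches the door mesh's world location, and the overlap event checks the actor's exact class and a DoorOpened boolean so the opening cannot retrigger.
; A timeline then drives a Lerp on world Z to raise the mesh by a fixed offset, with no closing logic.
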(event OnComponentBeginOverlap(CollisionBox)
  (params (OverlappedComponent :type Primitive%20Component%20Object%20Reference) (OtherActor :type Actor%20Object%20Reference) (OtherComp :type Primitive%20Component%20Object%20Reference) (OtherBodyIndex :type Integer) (bFromSweep :type Boolean) (SweepResult :type Hit%20Result%20Structure%20%28by%20ref%29))
  (bind _doorstartinglocation (Variables|Default|GetDoorStartingLocation))
  (if (== (Utilities|GetClass OtherActor) "/Game/FirstPerson/Blueprints/BP_FirstPersonCharacter.BP_FirstPersonCharacter_C")
    (if (not (Variables|Default|GetDoorOpened))
      (Variables|Default|SetDoorOpened true)
      (bind _dooropeninglerp (Timeline|BooleanDoorSlideUp PlayFromStart)
        (:Update
          (Transformation|SetWorldLocation (Variables|Default|GetSM_BooleanDoor) (Math|Vector|MakeVector (.x _doorstartinglocation) (.y _doorstartinglocation) (Math|Float|Lerp (.z _doorstartinglocation) (+ (.z _doorstartinglocation) 601.0) _dooropeninglerp)) false false))))))

(event EventBeginPlay
  (Variables|Default|SetDoorStartingLocation (Transformation|GetWorldLocation (Variables|Default|GetSM_BooleanDoor))))

(fn ConstructionScript)