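; BP_StrafingSpikes is a hazard-style actor whose spike mesh rotates and slides between two points defined by scene components.
; On BeginPlay it targets RotatingMovement at the mesh and caches the start and end components' relative locations.
; After StrafingDelay, a timeline with play rate set by StrafingSpeed drives a vector lerp that moves the mesh in relative space, without sweep.
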(event EventBeginPlay
  (Components|Movement|SetUpdatedComponent (Variables|Default|GetRotatingMovement) (Variables|Default|GetSM_StraftingSpikes))
  (Variables|Default|SetSpikesStartingLocation (Variables|/Script/Engine.SceneComponent|GetRelativeLocation (Variables|Default|GetSpikeStartingLoc)))
  (Variables|Default|SetSpikesEndingLocation (Variables|/Script/Engine.SceneComponent|GetRelativeLocation (Variables|Default|GetSpikeEndingLoc)))
  (Components|Timeline|SetPlayRate (Variables|Default|GetSpikesLocationTimeline) (Variables|Default|GetStrafingSpeed))
  (Utilities|FlowControl|Delay (Variables|Default|GetStrafingDelay))
  (bind _spikelocationalpha (Timeline|SpikesLocationTimeline PlayFromStart)
    (:Update
      (Transformation|SetRelativeLocation (Variables|Default|GetSM_StraftingSpikes) (Math|Vector|Lerp(Vector) (Variables|Default|GetSpikesStartingLocation) (Variables|Default|GetSpikesEndingLocation) _spikelocationalpha) false false))))

(fn ConstructionScript)