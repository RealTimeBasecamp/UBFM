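; A swinging blade hazard actor that rocks its blade mesh back and forth on the roll axis.
; The construction script tilts the mesh to one extreme by the rotation amount, and BeginPlay records that starting rotation.
; After a per-instance delay that lets multiple blades swing out of sync, a timeline with adjustable play rate lerps roll to the opposite extreme, keeping pitch and yaw fixed.
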(event EventBeginPlay
  ;[0.05729 0.05729 0.05729 0.5] Initialise Rotation Values
  (Components|Timeline|SetPlayRate (Variables|Default|GetBladesRoationTimeline) (Variables|Default|GetRotationSpeed))
  (Variables|Default|SetStartingRelativeRotation (Variables|/Script/Engine.SceneComponent|GetRelativeRotation (Variables|Default|GetSM_SwingingBlades)))
  ;[0.0382 0.6445 0 0.5] Offset Multiple Blades Using Delay
  (Utilities|FlowControl|Delay (Variables|Default|GetRotationDelay))
  ;[0 0.3864 0.8796 0.5] Setting Relative Rotation
  (bind _bladesrotationalpha (Timeline|BladesRoationTimeline PlayFromStart)
    (:Update
      (Transformation|SetRelativeRotation (Variables|Default|GetSM_SwingingBlades) (Math|Rotator|MakeRotator (Math|Float|Lerp (.roll (Variables|Default|GetStartingRelativeRotation)) (+ (.roll (Variables|Default|GetStartingRelativeRotation)) (* (Variables|Default|GetRotationAmount) -2.0)) _bladesrotationalpha) (.pitch (Variables|Default|GetStartingRelativeRotation)) (.yaw (Variables|Default|GetStartingRelativeRotation))) false false))))

(fn ConstructionScript
  (bind _sm_swingingblades (Variables|Default|GetSM_SwingingBlades))
  (bind _relativerotation (Variables|/Script/Engine.SceneComponent|GetRelativeRotation _sm_swingingblades))
  ;[0 0.3968 0.8963 0.5] Setting up inital relative rotation
  (Transformation|SetRelativeRotation _sm_swingingblades (Math|Rotator|MakeRotator (Variables|Default|GetRotationAmount) (.pitch _relativerotation) (.yaw _relativerotation)) false false))