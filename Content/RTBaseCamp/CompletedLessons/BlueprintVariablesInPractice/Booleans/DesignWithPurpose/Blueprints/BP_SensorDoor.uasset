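; BP_SensorDoor is a lesson door that opens when the first-person character enters its sensor box while the door is unlockable and the player has the key.
; On begin overlap, it checks the actor's exact class, then its own two booleans.
; Opening hides the door mesh and disables its collision; a failed check restores both.
; No end-overlap handler exists, so leaving the box does not close it.
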(event OnComponentBeginOverlap(SensorAreaCollisionBox)
  (params (OverlappedComponent :type Primitive%20Component%20Object%20Reference) (OtherActor :type Actor%20Object%20Reference) (OtherComp :type Primitive%20Component%20Object%20Reference) (OtherBodyIndex :type Integer) (bFromSweep :type Boolean) (SweepResult :type Hit%20Result%20Structure%20%28by%20ref%29))
  (bind _sm_door (Variables|Default|GetSM_Door))
  ;[0.2831 0 0] Checking if player overlaps sensor collions box
  (if (== (Utilities|GetClass OtherActor) "/Game/FirstPerson/Blueprints/BP_FirstPersonCharacter.BP_FirstPersonCharacter_C")
    ;[0.2961 0 0] Checks if the player has the key
    (if (and (Variables|Default|GetDoorUnlockable) (Variables|Default|GetHasPlayerGotKey))
      ;[0 0.3864 0.8714 0.5] Unlock/Lock door
      (Rendering|SetVisibility _sm_door false true)
      (Collision|SetCollisionEnabled _sm_door "NoCollision")
      (else
        (Rendering|SetVisibility _sm_door true true)
        (Collision|SetCollisionEnabled _sm_door "QueryAndPhysics")))))

(fn ConstructionScript)