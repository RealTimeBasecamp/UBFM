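; Blockout vault door Actor that slides open and closed through its DoorOpening event, driven by a boolean.
; A Timeline, sped up in the Construction Script, plays or reverses to lerp the door mesh between its BeginPlay relative location and a fixed open position.
; A referenced warning light activates when movement starts and switches off when the Timeline finishes.
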(event Custom|DoorOpening
  (params (IsDoorOpening? :type Boolean))
  (bind _bp_warninglightref (Variables|Default|GetBP_WarningLightRef))
  (if IsDoorOpening?
    (Default|ActivateLight _bp_warninglightref true)
    (bind _pressureplatealpha (Timeline|Timeline Play)
      (:Update
        (Transformation|SetRelativeLocation (Variables|Default|GetSM_Door) (Math|Vector|Lerp(Vector) (Variables|Default|GetRelative%20Location) "0.000000,1300.000000,0.000000" _pressureplatealpha) false false))
      (:Finished
        (Default|ActivateLight _bp_warninglightref false)))
    (else
      (Default|ActivateLight _bp_warninglightref true)
      (Timeline|Timeline Reverse))))

(event EventBeginPlay
  (Variables|Default|SetRelative%20Location (Variables|/Script/Engine.SceneComponent|GetRelativeLocation (Variables|Default|GetSM_Door))))

(fn ConstructionScript
  (Components|Timeline|SetPlayRate (Variables|Default|GetTimeline) 1.5))