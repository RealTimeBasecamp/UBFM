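; BP_PressurePlateBO is a pressure plate that opens a referenced vault door while its collision box is overlapped.
; Begin and end overlap call DoorOpening on VaultDoorRef with true or false, with no filter on the overlapping actor.
; The same events play and reverse a timeline, sped up in the construction script, that lerps the plate mesh between its BeginPlay relative location and a fixed, pressed offset.
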(event OnComponentBeginOverlap(CollisionBox)
  (params (OverlappedComponent :type Primitive%20Component%20Object%20Reference) (OtherActor :type Actor%20Object%20Reference) (OtherComp :type Primitive%20Component%20Object%20Reference) (OtherBodyIndex :type Integer) (bFromSweep :type Boolean) (SweepResult :type Hit%20Result%20Structure%20%28by%20ref%29))
  (Default|DoorOpening (Variables|Default|GetVaultDoorRef) true)
  (bind _pressureplatealpha (Timeline|Timeline Play)
    (:Update
      (Transformation|SetRelativeLocation (Variables|Default|GetSM_PressurePlate) (Math|Vector|Lerp(Vector) (Variables|Default|GetRelative%20Location) "0.000000,0.000000,-0.500000" _pressureplatealpha) false false))))

(event OnComponentEndOverlap(CollisionBox)
  (params (OverlappedComponent :type Primitive%20Component%20Object%20Reference) (OtherActor :type Actor%20Object%20Reference) (OtherComp :type Primitive%20Component%20Object%20Reference) (OtherBodyIndex :type Integer))
  (Default|DoorOpening (Variables|Default|GetVaultDoorRef) false)
  (bind _pressureplatealpha (Timeline|Timeline Reverse)
    (:Update
      (Transformation|SetRelativeLocation (Variables|Default|GetSM_PressurePlate) (Math|Vector|Lerp(Vector) (Variables|Default|GetRelative%20Location) "0.000000,0.000000,-0.500000" _pressureplatealpha) false false))))

(event EventBeginPlay
  (Variables|Default|SetRelative%20Location (Variables|/Script/Engine.SceneComponent|GetRelativeLocation (Variables|Default|GetSM_PressurePlate))))

(fn ConstructionScript
  (Components|Timeline|SetPlayRate (Variables|Default|GetTimeline) 1.5))