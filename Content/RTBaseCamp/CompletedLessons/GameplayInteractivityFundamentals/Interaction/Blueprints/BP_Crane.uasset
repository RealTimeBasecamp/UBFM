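; BP_Crane is an interactable crane that blends the player's camera to itself and can slide its Cube along an X track.
; Interact and a pressed-key CraneXUpdate both trigger the cubic view-target blend, while key release clears Xforward.
; While Xforward is set, Tick lerps the Cube between start and end markers cached at BeginPlay, using a per-frame step.
; The nodes that set Xforward true are disconnected.
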(event EventTick
  (params (DeltaSeconds :type Float%20%28single-precision%29))
  (if (Variables|Default|GetXforward)
    (Variables|Default|SetXLerpLoc (Math|Float|Clamp(Float) (+ (Variables|Default|GetXLerpLoc) 1e-05)))
    (Transformation|SetWorldLocation (Variables|Default|GetCube) (Math|Vector|Lerp(Vector) (Variables|Default|GetXStartLocation) (Variables|Default|GetXEndLocation) (Variables|Default|GetXLerpLoc)) false false)))

(event EventCraneXUpdate
  (params (ForwardKeyDown :type Boolean))
  (if ForwardKeyDown
    (Game|Player|SetViewTargetwithBlend (Game|GetPlayerController 0) self 5.0 "VTBlend_Cubic" 0.0 false)
    (else
      (Variables|Default|SetXforward false))))

(event EventBeginPlay
  (Variables|Default|SetXStartLocation (Transformation|GetWorldLocation (Variables|Default|GetXStartLoc)))
  (Variables|Default|SetXEndLocation (Transformation|GetWorldLocation (Variables|Default|GetXEndLoc))))

(event EventInteract
  (Game|Player|SetViewTargetwithBlend (Game|GetPlayerController 0) self 5.0 "VTBlend_Cubic" 0.0 false))

(fn ConstructionScript)