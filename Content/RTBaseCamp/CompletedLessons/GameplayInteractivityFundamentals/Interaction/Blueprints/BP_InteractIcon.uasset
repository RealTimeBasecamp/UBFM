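; BP_InteractIcon is a text prompt actor that signals when an interaction is available.
; Every tick it rotates to face opposite the player camera's forward vector, acting as a billboard.
; The text starts hidden; OverlapInteract shows or hides it according to its Overlapping flag.
; While shown, a Timeline drives the text colour between TextColour1 and TextColour2, and hiding the text stops it.
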(event EventOverlapInteract
  (params (Overlapping :type Boolean))
  (bind _textrender (Variables|Default|GetTextRender))
  (if Overlapping
    (Rendering|SetVisibility _textrender true false)
    (bind _newtrack_0 (Timeline|Timeline PlayFromStart)
      (:Update
        (Rendering|Components|TextRender|SetTextRenderColor (Variables|Default|GetTextRender) (Math|Conversions|ToColor(LinearColor) (Math|Color|Lerp(LinearColor) (Math|Conversions|ToLinearColor(Color) (Variables|Default|GetTextColour1)) (Math|Conversions|ToLinearColor(Color) (Variables|Default|GetTextColour2)) _newtrack_0)))))
    (else
      (Rendering|SetVisibility _textrender false false)
      (Timeline|Timeline Stop))))

(event EventBeginPlay
  (Rendering|SetVisibility (Variables|Default|GetTextRender) false false))

(event EventTick
  (params (DeltaSeconds :type Float%20%28single-precision%29))
  (Transformation|SetActorRotation (Math|Conversions|RotationFromXVector (* (Math|Vector|GetForwardVector (Camera|GetCameraRotation (Game|GetPlayerCameraManager 0))) "-1.000000,-1.000000,-1.000000"))))

(fn ConstructionScript)