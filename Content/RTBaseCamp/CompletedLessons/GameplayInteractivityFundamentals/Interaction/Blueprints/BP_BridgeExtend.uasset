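; BP_BridgeExtend is an interactable bridge for a gameplay interactivity lesson that extends once when triggered.
; The construction script caches the Cube's world scale as the starting value.
; On the first Interact event, a boolean latches and a Timeline lerps the Cube's X world scale to a hardcoded length, keeping Y and Z unchanged.
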(event EventInteract
  (bind _currentworldscale (Variables|Default|GetCurrentWorldScale))
  (bind (_x _y _z) (Math|Vector|BreakVector _currentworldscale))
  (if (not (Variables|Default|GetHasExtended))
    (Variables|Default|SetHasExtended true)
    (bind _newtrack_0 (Timeline|Timeline PlayFromStart)
      (:Update
        (Transformation|SetWorldScale3D (Variables|Default|GetCube) (Math|Vector|Lerp(Vector) _currentworldscale (Math|Vector|MakeVector 14.0 _y _z) _newtrack_0))))))

(fn ConstructionScript
  (Variables|Default|SetCurrentWorldScale (Transformation|GetWorldScale (Variables|Default|GetCube))))