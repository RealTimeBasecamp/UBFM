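; Control panel actor with a button the player can press while inside its collision sphere to trigger a set of target actors.
; On Interact, it confirms the overlap, briefly scales up the button mesh, then sends InteractMessage to each entry in the Target array.
; Sphere overlaps notify the child interact icon, enabling its tick on begin, while end overlap disables tick on the panel itself.
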(event OnComponentBeginOverlap(ButtonCollisionSphere)
  (params (OverlappedComponent :type Primitive%20Component%20Object%20Reference) (OtherActor :type Actor%20Object%20Reference) (OtherComp :type Primitive%20Component%20Object%20Reference) (OtherBodyIndex :type Integer) (bFromSweep :type Boolean) (SweepResult :type Hit%20Result%20Structure%20%28by%20ref%29))
  (bind _bp_interacticon (Variables|Default|GetBP_InteractIcon))
  (bind _childactor (Variables|/Script/Engine.ChildActorComponent|GetChildActor _bp_interacticon))
  (Class|BPIInteract|OverlapInteract(Message) _childactor true)
  (Actor|Tick|SetActorTickEnabled _childactor true))

(event OnComponentEndOverlap(ButtonCollisionSphere)
  (params (OverlappedComponent :type Primitive%20Component%20Object%20Reference) (OtherActor :type Actor%20Object%20Reference) (OtherComp :type Primitive%20Component%20Object%20Reference) (OtherBodyIndex :type Integer))
  (Class|BPIInteract|OverlapInteract(Message) (Variables|/Script/Engine.ChildActorComponent|GetChildActor (Variables|Default|GetBP_InteractIcon)) false)
  (Actor|Tick|SetActorTickEnabled false))

(event EventInteract
  (bind _sm_controlpannelsinglebutton (Variables|Default|GetSM_ControlPannelSingleButton))
  (if (Collision|IsOverlappingActor (Variables|Default|GetButtonCollisionSphere) (Game|Player|GetPlayerPawn 0) :!class /Script/Engine.PrimitiveComponent)
    (Transformation|SetWorldScale3D _sm_controlpannelsinglebutton (* (Transformation|GetWorldScale _sm_controlpannelsinglebutton) "1.500000,1.500000,1.500000"))
    (Utilities|FlowControl|Delay 0.2)
    (Transformation|SetWorldScale3D _sm_controlpannelsinglebutton "1.000000,1.000000,1.000000")
    (for _array_element (Variables|Default|GetTarget)
      (Class|BPIInteract|Interact(Message) _array_element))))

(fn ConstructionScript)