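; BP_SwingingSpikes is a spike obstacle that swings around a pivot along the roll axis.
; The construction script tilts RotationPivot to RotationAmount and sets the timeline play rate from RotationSpeed.
; On BeginPlay it stores that starting rotation, waits RotateDelay, then plays RotateBladeTimeline.
; Each update lerps roll from the start toward the mirrored negative angle using the timeline curve, leaving pitch and yaw unchanged.
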(event EventBeginPlay
  (Variables|Default|SetStartingRelativeRotation (Variables|/Script/Engine.SceneComponent|GetRelativeRotation (Variables|Default|GetRotationPivot)))
  (Utilities|FlowControl|Delay (Variables|Default|GetRotateDelay))
  (bind _slidingspikescale (Timeline|RotateBladeTimeline PlayFromStart)
    (:Update
      (Transformation|SetRelativeRotation (Variables|Default|GetRotationPivot) (Math|Rotator|MakeRotator (Math|Float|Lerp (.roll (Variables|Default|GetStartingRelativeRotation)) (+ (.roll (Variables|Default|GetStartingRelativeRotation)) (* (Variables|Default|GetRotationAmount) -2.0)) _slidingspikescale) (.pitch (Variables|Default|GetStartingRelativeRotation)) (.yaw (Variables|Default|GetStartingRelativeRotation))) false false))))

(fn ConstructionScript
  (bind _rotationpivot (Variables|Default|GetRotationPivot))
  (bind _relativerotation (Variables|/Script/Engine.SceneComponent|GetRelativeRotation _rotationpivot))
  (Transformation|SetRelativeRotation _rotationpivot (Math|Rotator|MakeRotator (Variables|Default|GetRotationAmount) (.pitch _relativerotation) (.yaw _relativerotation)) false false)
  (Components|Timeline|SetPlayRate (Variables|Default|GetRotateBladeTimeline) (Variables|Default|GetRotationSpeed)))