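; BP_SplineLanterns is a spline lesson actor that builds a string of meshes, by its name lanterns, along an editable spline.
; The Construction Script adds hierarchical instanced meshes at every spline point and static mesh components evenly spaced by distance, using NoOfInstances.
; The same count-driven loop adds uniformly scaled spline meshes between consecutive point indices, independent of the actual point count.
; The Event Graph holds only an unconnected SpawnActor node.
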(fn ConstructionScript
  (bind _spline (Variables|Default|GetSpline))
  (bind _noofinstances (Variables|Default|GetNoOfInstances))
  (bind _newvar_0 (Variables|Default|GetNewVar_0))
  (for _index (range 0 (- (Spline|GetNumberOfSplinePoints _spline) 1))
    (Utilities|Array|Add (Variables|Default|GetNewVar) (Spline|GetTransformatSplinePoint _spline _index "Local" false)))
  (Components|InstancedStaticMesh|AddInstances (Variables|Default|GetHierarchicalInstancedStaticMesh) (Variables|Default|GetNewVar) false false)
  (for _index_2 (range 0 _noofinstances)
    (AddComponent|AddStaticMeshComponent false (Math|Transform|MakeTransform (Spline|GetLocationatDistanceAlongSpline _spline (* (/ (Spline|GetSplineLength _spline) _noofinstances) _index_2) "Local") "0, 0, 0" "1.000000,1.000000,1.000000"))
    (bind _returnvalue (AddComponent|AddSplineMeshComponent false))
    (SplineMesh|SetStartandEnd _returnvalue (.Location (Spline|GetLocationandTangentatSplinePoint _spline _index_2 "Local")) (.Tangent (Spline|GetLocationandTangentatSplinePoint _spline _index_2 "Local")) (.Location (Spline|GetLocationandTangentatSplinePoint _spline (+ _index_2 1) "Local")) (.Tangent (Spline|GetLocationandTangentatSplinePoint _spline (+ _index_2 1) "Local")) true :!class /Script/Engine.SplineMeshComponent)
    (SplineMesh|SetEndScale _returnvalue (Math|Vector2D|MakeVector2D _newvar_0 _newvar_0) true :!class /Script/Engine.SplineMeshComponent)
    (SplineMesh|SetStartScale _returnvalue (Math|Vector2D|MakeVector2D _newvar_0 _newvar_0) true :!class /Script/Engine.SplineMeshComponent)))