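; A reference Blueprint from a base camp lesson set that showcases Unreal variable types, from primitives, enums and structs to object references and containers.
; The event graph is a gallery of unconnected example nodes for literals, conversions, boolean logic, math, string operations, switches and branches, none of which run.
; Only the Construction Script executes, printing the length of an integer array, beside a few more unused boolean and conversion examples.
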(fn ConstructionScript
  (Development|PrintString (Utilities|String|ToString(Integer) (Utilities|Array|Length (Utilities|Array|MakeArray (Variables|Default|GetInt))))))