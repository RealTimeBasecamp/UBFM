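; BP_TrophySpline is an actor that displays a configurable row of trophies with 3D text labels along a spline.
; Its construction script resizes TrophyData to NoOfTrophies, then spawns static meshes evenly spaced from end to end of BottomSpline.
; Each entry supplies metal and emissive materials for both mesh and text, plus the label, height offset and size.
; A flag sets whether RotatingMovement auto-activates, and the event graph is unused.
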(event EventBeginPlay)

(event Collision|EventActorBeginOverlap
  (params (OtherActor :type Actor%20Object%20Reference)))

(event EventTick
  (params (DeltaSeconds :type Float%20%28single-precision%29)))

(fn ConstructionScript
  (bind _nooftrophies (Variables|Default|GetNoOfTrophies))
  (bind _trophyscalemultiplier (Variables|Default|GetTrophyScaleMultiplier))
  (Utilities|Array|Resize (Variables|Default|GetTrophyData) _nooftrophies)
  (for _index (range 0 (- _nooftrophies 1))
    (bind _returnvalue (AddComponent|AddStaticMeshComponent true))
    (bind _output_get (LocalVariables|SetCurrentTrophy _returnvalue))
    (Transformation|SetRelativeScale3D _output_get (Math|Vector|MakeVector _trophyscalemultiplier _trophyscalemultiplier _trophyscalemultiplier))
    (Transformation|SetWorldLocation _returnvalue (Spline|GetLocationatDistanceAlongSpline (Variables|Default|GetBottomSpline) (* _index (/ (Spline|GetSplineLength (Variables|Default|GetBottomSpline)) (- _nooftrophies 1))) "World") false true)
    (Rendering|Material|SetMaterial _returnvalue 0 (.TrophyMetalMat (Utilities|Struct|BreakSTrophyData (Utilities|Array|Get(acopy) (Variables|Default|GetTrophyData) _index))))
    (Rendering|Material|SetMaterial _returnvalue 1 (.TrophyEmissiveMat (Utilities|Struct|BreakSTrophyData (Utilities|Array|Get(acopy) (Variables|Default|GetTrophyData) _index))))
    (bind _returnvalue_2 (AddComponent|AddText3DComponent false))
    (Components|Activation|SetAutoActivate (Variables|Default|GetRotatingMovement) (Variables|Default|GetIsRotating))
    (Transformation|SetRelativeRotation _returnvalue_2 (Math|Rotator|MakeRotator 0.0 0.0 (Variables|Default|GetTextRotationOffset)) false false)
    (Class|Text3DComponent|SetText _returnvalue_2 (Utilities|Text|ToText(String) (Utilities|String|Replace (.TrophyText (Utilities|Struct|BreakSTrophyData (Utilities|Array|Get(acopy) (Variables|Default|GetTrophyData) _index))) " " " 
")))
    (Class|Text3DComponent|SetFreeze _returnvalue_2 true)
    (Class|Text3DComponent|SetBackMaterial _returnvalue_2 (.TrophyMetalMat (Utilities|Struct|BreakSTrophyData (Utilities|Array|Get(acopy) (Variables|Default|GetTrophyData) _index))))
    (Class|Text3DComponent|SetFrontMaterial _returnvalue_2 (.TrophyMetalMat (Utilities|Struct|BreakSTrophyData (Utilities|Array|Get(acopy) (Variables|Default|GetTrophyData) _index))))
    (Class|Text3DComponent|SetBevelMaterial _returnvalue_2 (.TrophyEmissiveMat (Utilities|Struct|BreakSTrophyData (Utilities|Array|Get(acopy) (Variables|Default|GetTrophyData) _index))))
    (Class|Text3DComponent|SetExtrudeMaterial _returnvalue_2 (.TrophyEmissiveMat (Utilities|Struct|BreakSTrophyData (Utilities|Array|Get(acopy) (Variables|Default|GetTrophyData) _index))))
    (Transformation|SetWorldLocation _returnvalue_2 (Math|Vector|MakeVector (.x (Transformation|GetWorldLocation (LocalVariables|GetCurrentTrophy))) (.y (Transformation|GetWorldLocation (LocalVariables|GetCurrentTrophy))) (+ (.z (Transformation|GetWorldLocation (LocalVariables|GetCurrentTrophy))) (* (.ZOffset (Utilities|Struct|BreakSTrophyData (Utilities|Array|Get(acopy) (Variables|Default|GetTrophyData) _index))) (Variables|Default|GetTrophyScaleMultiplier)))) false true)
    (Transformation|SetWorldScale3D _returnvalue_2 (* (Transformation|GetWorldScale _returnvalue_2) (Math|Vector|MakeVector (.TextSizeMultiplier (Utilities|Struct|BreakSTrophyData (Utilities|Array|Get(acopy) (Variables|Default|GetTrophyData) _index))) (.TextSizeMultiplier (Utilities|Struct|BreakSTrophyData (Utilities|Array|Get(acopy) (Variables|Default|GetTrophyData) _index))) (.TextSizeMultiplier (Utilities|Struct|BreakSTrophyData (Utilities|Array|Get(acopy) (Variables|Default|GetTrophyData) _index))))))))